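; Boss enemy that fights the player with randomly chosen horizontal or vertical melee montages and a hitbox that damages once per activation.
; Tick polls the player's round to raise speed and set battle state on the AI Blackboard, mirroring shield state there too.
; Shield state also drives material and idle rotation, while zero health triggers the AnimBP death flag.
; A sphere trigger controls AI focus, and killing the player raises the shield.
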(event OnComponentBeginOverlap(Box)
  (params (OverlappedComponent :type Primitive%20Component%20Object%20Reference) (OtherActor :type Actor%20Object%20Reference) (OtherComp :type Primitive%20Component%20Object%20Reference) (OtherBodyIndex :type Integer) (bFromSweep :type Boolean) (SweepResult :type Hit%20Result%20Structure%20%28by%20ref%29))
  (bind _ref_bp_character_base (Variables|Default|GetRef%20BP%20Character%20Base))
  (if (Variables|Default|GetActive?)
    (bind _asbp_character_base (Utilities|Casting|CastToBP_CharacterBase OtherActor))
    (Game|Damage|ApplyDamage _asbp_character_base 5e+01 0 0)
    (Variables|Default|SetDeath (== (Class|CharacterBase|GetHealthPercent _asbp_character_base) 0.0))
    (Variables|Default|SetActive? false)
    (if (== (Class|CharacterBase|GetHealthPercent _ref_bp_character_base) 0.0)
      (Default|Dead _ref_bp_character_base)
      (Class|Enemy|VShield true))))

(event OnComponentBeginOverlap(Sphere)
  (params (OverlappedComponent :type Primitive%20Component%20Object%20Reference) (OtherActor :type Actor%20Object%20Reference) (OtherComp :type Primitive%20Component%20Object%20Reference) (OtherBodyIndex :type Integer) (bFromSweep :type Boolean) (SweepResult :type Hit%20Result%20Structure%20%28by%20ref%29))
  (bind _self self)
  (bind _returnvalue (AI|GetAIController _self))
  (bind _asbp_character_base (Utilities|Casting|CastToBP_CharacterBase OtherActor))
  (if (not (Class|Enemy|GetShield))
    (Utilities|IsValid _returnvalue
      (:Is%20Valid
        (AI|SetFocus _returnvalue _asbp_character_base)))))

(event OnComponentEndOverlap(Sphere)
  (params (OverlappedComponent :type Primitive%20Component%20Object%20Reference) (OtherActor :type Actor%20Object%20Reference) (OtherComp :type Primitive%20Component%20Object%20Reference) (OtherBodyIndex :type Integer))
  (bind _self self)
  (bind _returnvalue (AI|GetAIController _self))
  (Utilities|Casting|CastToBP_CharacterBase OtherActor)
  (Utilities|IsValid _returnvalue
    (:Is%20Valid
      (AI|ClearFocus _returnvalue))))

(event Custom|Damage
  (params (bActive :type Boolean))
  (Variables|Default|SetActive? bActive))

(event EventBeginPlay
  (bind _asbp_character_base (Utilities|Casting|CastToBP_CharacterBase (Game|Player|GetPlayerPawn 0)))
  (Variables|Default|SetRef%20BP%20Character%20Base _asbp_character_base))

(event EventMeleeAttack
  (bind _mesh (Variables|Character|GetMesh))
  (if (not (Variables|Default|GetDeath))
    (if (Math|Random|RandomBool)
      (Animation|Montage|PlayMontage _mesh "/Game/Boss/Animations/M_AttackHorizontal.M_AttackHorizontal" 1.5)
      (else
        (Animation|Montage|PlayMontage _mesh "/Game/Boss/Animations/M_AttackVertical.M_AttackVertical" 1.5)))))

(event EventTick
  (params (DeltaSeconds :type Float%20%28single-precision%29))
  (bind _returnvalue (Class|Enemy|GetShield))
  (bind _returnvalue_2 (AI|GetBlackboard 0))
  (bind _returnvalue_3 (AI|GetBlackboard 0))
  (bind _mesh (Variables|Character|GetMesh))
  (Utilities|FlowControl|Sequence
    (:then_0
      (if (== (Class|CharacterBase|GetNowRound (Variables|Default|GetRef%20BP%20Character%20Base)) 2)
        (Variables|/Script/Engine.CharacterMovementComponent|SetMaxWalkSpeed (Variables|Character|GetCharacterMovement) 6e+02)
        (Utilities|IsValid _returnvalue_3
          (:Is%20Valid
            (AI|Components|Blackboard|SetValueasBool _returnvalue_3 (Utilities|Name|MakeLiteralName "BattleBoss") true)))))
    (:then_1
      (Utilities|IsValid _returnvalue_2
        (:Is%20Valid
          (AI|Components|Blackboard|SetValueasBool _returnvalue_2 (Utilities|Name|MakeLiteralName "BattleBossShield") _returnvalue))
        (:Is%20Not%20Valid
          _))
      (if (and _returnvalue (== (Math|Vector|VectorLength (Transformation|GetVelocity)) 0.0))
        (Transformation|SetActorRotation "0, 0, 0")
        (elif (Class|Enemy|GetShield)
          (if (not (<= (Class|CharacterBase|GetHealthPercent (Variables|Default|GetRef%20BP%20Character%20Base)) 0.0))
            (Rendering|Material|SetMaterial _mesh 0 "/Game/Boss/BossTexture1.BossTexture1"))
          (else
            (Rendering|Material|SetMaterial _mesh 0 "/Game/Boss/BossTexture.BossTexture")))))
    (:then_2
      (if (<= (Class|Enemy|GetHealthPercent) 0.0)
        (bind _asanim_boss (Utilities|Casting|CastToAnim_Boss (Components|SkeletalMesh|GetAnimInstance (Variables|Character|GetMesh))))
        (Variables|/Game/_Blueprint/Enemy/Anim_Boss/Anim_Boss.Anim_Boss_C|SetDeath _asanim_boss true)))))

(fn ConstructionScript)