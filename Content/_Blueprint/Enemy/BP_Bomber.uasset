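; BP_Bomber is an enemy Blueprint that tracks its death state and drives a health widget.
; BeginPlay caches the player pawn as a BP_CharacterBase reference, which the event graph does not use further.
; Tick polls GetHealthPercent into the W_HealthBoom widget; at exactly zero it sets Dead and hides the widget component after a short Delay.
; The graph contains no movement, attack or explosion logic.
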(event EventBeginPlay
  (bind _asbp_character_base (Utilities|Casting|CastToBP_CharacterBase (Game|Player|GetPlayerPawn 0)))
  (Variables|Default|SetRef%20BP%20Character%20Base _asbp_character_base))

(event Collision|EventActorBeginOverlap
  (params (OtherActor :type Actor%20Object%20Reference)))

(event EventTick
  (params (DeltaSeconds :type Float%20%28single-precision%29))
  (bind _returnvalue (Class|Enemy|GetHealthPercent))
  (bind _asw_health_boom (Utilities|Casting|CastToW_HealthBoom (UserInterface|GetUserWidgetObject (Variables|Default|GetWidget))))
  (Variables|/Game/_Blueprint/Widget/W_HealthBoom.W_HealthBoom_C|SetHealth _asw_health_boom _returnvalue)
  (if (== _returnvalue 0.0)
    (Variables|Default|SetDead true)
    (Utilities|FlowControl|Delay 0.5)
    (Rendering|SetVisibility (Variables|Default|GetWidget) false false)))

(fn ConstructionScript)