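; Spawner that runs alternating bomber-wave and boss rounds, polling the player's round every second.
; Odd rounds check Ver to restore health and open the boss fight by dropping its shield; Ver's kill-quota comparison is unconnected.
; In rounds 2 and 4, boss health thresholds restore the shield and call Begin.
; Begin spawns AI bombers around every TargetPointsBoom, with count and speed set by round.
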(event Custom|Begin
  (for _index (range 1 (Utilities|Array|Get(acopy) (Variables|Default|GetBoomRound) (Class|CharacterBase|GetNowRound (Variables|Default|GetRef%20BP%20Character%20Base))))
    (bind _outactors (Actor|GetAllActorsOfClass "/Game/_Blueprint/Map/TargetPointsBoom.TargetPointsBoom_C"))
    (for _array_element _outactors
      (bind _returnvalue (AI|SpawnAIFromClass "/Game/_Blueprint/Enemy/BP_Bomber.BP_Bomber_C" "/Game/_Blueprint/Enemy/AI_Bomber/BT_Bomber.BT_Bomber" (Math|Random|RandomPointinBoundingBox (Transformation|GetActorLocation _array_element) "100.000000,100.000000, 0") "0, 0, 0" true 0))
      (bind _asbp_bomber (Utilities|Casting|CastToBP_Bomber _returnvalue))
      (Variables|/Script/Engine.CharacterMovementComponent|SetMaxWalkSpeed (Variables|/Script/Engine.Character|GetCharacterMovement _asbp_bomber) (+ (Variables|/Script/Engine.CharacterMovementComponent|GetMaxWalkSpeed (Variables|/Script/Engine.Character|GetCharacterMovement _asbp_bomber)) (Math|Conversions|ToFloat(Integer) (* (Class|CharacterBase|GetNowRound (Variables|Default|GetRef%20BP%20Character%20Base)) 100)))))))

(event Custom|CheckRound
  (bind _ref_bp_character_base (Variables|Default|GetRef%20BP%20Character%20Base))
  (bind _ref_bp_character_base_2 (Variables|Default|GetRef%20BP%20Character%20Base))
  (bind _ref_bp_character_base_3 (Variables|Default|GetRef%20BP%20Character%20Base))
  (bind _returnvalue (Class|CharacterBase|GetNowRound _ref_bp_character_base))
  (bind _returnvalue_2 (Class|CharacterBase|GetNowRound _ref_bp_character_base_3))
  (bind _returnvalue_3 (Class|CharacterBase|GetNowRound _ref_bp_character_base_2))
  (if (Math|Boolean|ORBoolean (== _returnvalue_3 1) (== _returnvalue_3 3) (== _returnvalue_3 5))
    (if (|Ver)
      (Class|CharacterBase|VHealth (Variables|Default|GetRef%20BP%20Character%20Base) 1e+02)
      (Class|CharacterBase|VKill _ref_bp_character_base_3)
      (Class|CharacterBase|VNowRound _ref_bp_character_base_3 1)
      (if (Math|Boolean|ORBoolean (== _returnvalue_2 2) (== _returnvalue_2 4) (== _returnvalue_2 6))
        (Class|CharacterBase|VBattleBoss _ref_bp_character_base_3 true)
        (Class|Enemy|VShield (Variables|Default|GetRef%20Boss) false)))
    (elif (Math|Boolean|ORBoolean (== _returnvalue 2) (== _returnvalue 4) (== _returnvalue 6))
      (switch int _returnvalue
        (:2
          (if (<= (Class|Enemy|GetHealthPercent (Variables|Default|GetRef%20Boss)) 0.8)
            (Class|CharacterBase|VNowRound (Variables|Default|GetRef%20BP%20Character%20Base) 1)
            (Class|Enemy|VShield (Variables|Default|GetRef%20Boss) true)
            (CallFunction|Begin)))
        (:4
          (if (<= (Class|Enemy|GetHealthPercent (Variables|Default|GetRef%20Boss)) 0.6)
            (Class|CharacterBase|VNowRound (Variables|Default|GetRef%20BP%20Character%20Base) 1)
            (Class|Enemy|VShield (Variables|Default|GetRef%20Boss) true)
            (CallFunction|Begin)))))))

(event EventBeginPlay
  (bind _asbp_character_base (Utilities|Casting|CastToBP_CharacterBase (Game|Player|GetPlayerPawn 0)))
  (Variables|Default|SetRef%20BP%20Character%20Base _asbp_character_base)
  (bind _outactors (Actor|GetAllActorsOfClass "/Game/_Blueprint/Map/TargetPointsBoom.TargetPointsBoom_C"))
  (Variables|Default|SetNumTargetPoint (Utilities|Array|Length _outactors))
  (bind _outactors_2 (Actor|GetAllActorsOfClass "/Game/_Blueprint/Enemy/BP_Boss.BP_Boss_C"))
  (Variables|Default|SetRef%20Boss (Utilities|Array|Get(acopy) _outactors_2))
  (Utilities|Time|SetTimerbyEvent (delegate Custom|CheckRound) 1.0 true))

(fn ConstructionScript)