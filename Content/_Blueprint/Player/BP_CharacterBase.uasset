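; Player character Blueprint for a first-person shooter that handles pause, damage, death, kill counting and weapon feedback.
; BeginPlay caches the BP_Widget HUD, which pause and death update; zero health after damage opens the game-over widget.
; Tick polls GetHot and GetFire to swap the weapon's emissive material, play a one-shot overheat sound, and toggle muzzle particles and full-auto audio.
; Death hides the first-person mesh, weapon and HUD, then disables input.
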(event Custom|Dead
  (|N_Dead))

(event Custom|Kill
  (|N_Kill))

(event EventBeginPlay
  (|N_BeginPlay))

(event EventTick
  (params (DeltaSeconds :type Float%20%28single-precision%29))
  (|N_Tick))

(event Game|Damage|EventAnyDamage
  (params (Damage :type Float%20%28single-precision%29) (DamageType :type Damage%20Type%20Object%20Reference) (InstigatedBy :type Controller%20Object%20Reference) (DamageCauser :type Actor%20Object%20Reference))
  (|N_AnyDamage Damage))

(event Input|ActionEvents|InputActionPause
  (params (Key :type Key%20Structure :default "None"))
  (:Pressed
    (|N_Pause)))

(fn ConstructionScript)